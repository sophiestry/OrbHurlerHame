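; BP_PlayerPawn is a player pawn that moves by rolling physics torque on its static mesh and restarts the level when damaged.
; Forward/Backward and Left/Right axis inputs apply torque as an acceleration change, scaled by AccMultiplier.
; A collapsed Game Restart graph fades the camera in on BeginPlay; on any damage it fades out, waits, then reopens the current level by name.
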(event Collision|EventActorBeginOverlap
  (params (OtherActor :type Actor%20Object%20Reference)))

(event EventTick
  (params (DeltaSeconds :type Float%20%28single-precision%29)))

(event Game|Damage|EventAnyDamage
  (params (Damage :type Float%20%28single-precision%29) (DamageType :type Damage%20Type%20Object%20Reference) (InstigatedBy :type Controller%20Object%20Reference) (DamageCauser :type Actor%20Object%20Reference))
  (Utilities|GameRestart))

(event EventBeginPlay
  (Utilities|GameRestart) ; enters at execute2
)

(event Input|AxisEvents|InputAxisForward/Backward
  (params (AxisValue :type Float%20%28single-precision%29))
  (Class|PrimitiveComponent|AddTorqueinRadians (Variables|Default|GetStaticMesh) (Math|Vector|MakeVector 0.0 (* AxisValue (Variables|Default|GetAccMultiplier)) 0.0) "None" true))

(event Input|AxisEvents|InputAxisLeft/Right
  (params (AxisValue :type Float%20%28single-precision%29))
  (Class|PrimitiveComponent|AddTorqueinRadians (Variables|Default|GetStaticMesh) (Math|Vector|MakeVector (* AxisValue (Variables|Default|GetAccMultiplier)) 0.0 0.0) "None" true))

(fn ConstructionScript)